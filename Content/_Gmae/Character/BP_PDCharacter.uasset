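; BP_PDCharacter is a character Blueprint that serves as a test harness for jump montages and movement debugging.
; Keys 1–3 play run, walk and in-place jump montages from named sections, switching CharacterMovement to Flying during playback and back to Walking on completion, blend out or interruption.
; Tick draws ground-plane (Z=0) arrows for actor facing and aim yaw, and prints horizontal speed plus forward and right input values.
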(event EventTick
  (params (DeltaSeconds :type Float%20%28single-precision%29))
  (bind _returnvalue (Transformation|GetActorLocation))
  (bind _returnvalue_2 (Transformation|GetActorLocation))
  (bind _returnvalue_3 (Transformation|GetActorForwardVector))
  (bind _returnvalue_4 (Pawn|GetBaseAimRotation))
  (bind (_x _y) (Math|Vector|BreakVector _returnvalue_2))
  (bind _returnvalue_5 (Math|Vector|GetForwardVector (Math|Rotator|MakeRotator 0.0 0.0 (.yaw _returnvalue_4))))
  (bind _returnvalue_6 (* _returnvalue_3 1.5e+02))
  (bind _returnvalue_7 (* _returnvalue_5 1.5e+02))
  (bind _returnvalue_8 (+ (Math|Vector|MakeVector (.x _returnvalue) (.y _returnvalue) 0.0) _returnvalue_6))
  (bind _returnvalue_9 (+ _returnvalue_2 _returnvalue_7))
  (Rendering|Debug|DrawDebugArrow (Math|Vector|MakeVector (.x _returnvalue) (.y _returnvalue) 0.0) (Math|Vector|MakeVector (.x _returnvalue_8) (.y _returnvalue_8) 0.0) 3e+01 "(R=0.060576,G=0.000000,B=1.000000,A=1.000000)" 0.0 4.0)
  (Rendering|Debug|DrawDebugArrow (Math|Vector|MakeVector _x _y 0.0) (Math|Vector|MakeVector (.x _returnvalue_9) (.y _returnvalue_9) 0.0) 3e+01 "(R=1.000000,G=0.537374,B=0.000000,A=1.000000)" 0.0 4.0)
  (Development|PrintString (Utilities|String|Append "Speed : " (Utilities|String|ToString(Float) (Math|Vector|VectorLengthXY (Transformation|GetVelocity)))) true true "(R=1.000000,G=0.466965,B=0.000000,A=1.000000)" 0.0)
  (Development|PrintString (Utilities|String|Append "Right Input Value : " (Utilities|String|ToString(Float) (Variables|Default|GetRightInputValue))) true true "(R=0.000000,G=0.660000,B=1.000000,A=1.000000)" 0.0)
  (Development|PrintString (Utilities|String|Append "Forward Input Value : " (Utilities|String|ToString(Float) (Variables|Default|GetForwardInputValue))) true true "(R=0.000000,G=0.660000,B=1.000000,A=1.000000)" 0.0))

(event Input|KeyboardEvents|3
  (params (Key :type Key%20Structure :default "None"))
  (bind _charactermovement (Variables|Character|GetCharacterMovement))
  (:Pressed
    (Animation|Montage|PlayMontage (Variables|Character|GetMesh) "/Game/_Gmae/Character/Animation/Retarget/Jump/AM_JumpInPlace.AM_JumpInPlace" 1.0 0.0 "walk"
      (:then
        (Pawn|Components|CharacterMovement|SetMovementMode _charactermovement "MOVE_Flying" 0))
      (:OnCompleted
        (Pawn|Components|CharacterMovement|SetMovementMode _charactermovement "MOVE_Walking" 0 :!label _label))
      (:OnBlendOut
        (goto _label))
      (:OnInterrupted
        (goto _label)))))

(event Input|KeyboardEvents|1
  (params (Key :type Key%20Structure :default "None"))
  (bind _charactermovement (Variables|Character|GetCharacterMovement))
  (:Pressed
    (Animation|Montage|PlayMontage (Variables|Character|GetMesh) "/Game/_Gmae/Character/Animation/Retarget/Jump/AM_JumpRun.AM_JumpRun" 1.0 0.0 "right"
      (:then
        (Pawn|Components|CharacterMovement|SetMovementMode _charactermovement "MOVE_Flying" 0))
      (:OnCompleted
        (Pawn|Components|CharacterMovement|SetMovementMode _charactermovement "MOVE_Walking" 0 :!label _label))
      (:OnBlendOut
        (goto _label))
      (:OnInterrupted
        (goto _label)))))

(event Input|KeyboardEvents|2
  (params (Key :type Key%20Structure :default "None"))
  (bind _charactermovement (Variables|Character|GetCharacterMovement))
  (:Pressed
    (Animation|Montage|PlayMontage (Variables|Character|GetMesh) "/Game/_Gmae/Character/Animation/Retarget/Jump/AM_JumpWalk.AM_JumpWalk" 1.0 0.0 "stop"
      (:then
        (Pawn|Components|CharacterMovement|SetMovementMode _charactermovement "MOVE_Flying" 0))
      (:OnCompleted
        (Pawn|Components|CharacterMovement|SetMovementMode _charactermovement "MOVE_Walking" 0 :!label _label))
      (:OnBlendOut
        (goto _label))
      (:OnInterrupted
        (goto _label)))))

(fn ConstructionScript)